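; BP_NPC is an interactable NPC that prints a line of dialogue each time its Interact event fires.
; Interact increments DialogIndex, resets it to zero once it exceeds the Dialog array length, then shows that entry with PrintString.
; The increment precedes the read, and the bounds check lets the index equal the array length, one past the last entry.
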(event `/Game/Blueprints/BP_interface.Interact`
  (`/Engine/EditorBlueprintResources/StandardMacros.IncrementInt` (`self.DialogIndex`)
    (:`  `
      (if (not (<= (`self.DialogIndex`) (`KismetArrayLibrary.Array_Length` (`self.Dialog`))))
        (set `self.DialogIndex` 0))
      (`KismetSystemLibrary.PrintString` (`|GetArrayItem` (`self.Dialog`) (`self.DialogIndex`))))))

(fn `UserConstructionScript`)